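; Pickup item actor that spins in place and goes into the player's inventory on interaction.
; Interact calls DestroyActor first, then casts the player to BP_FirstPersonCharacter, passes Iteminfo to its Invenwidget's AddToInventory and calls DestroyActor again.
; UseItem only prints a debug string.
; Tick yaws the root by DeltaSeconds plus one degree each frame, so spin speed depends on frame rate.
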(event `/Game/blueprint/interface/interact.interact`
  (`self.K2_DestroyActor`)
  (bind _asbp_first_person_character (cast `/Game/blueprint/character/BP_FirstPersonCharacter` (`GameplayStatics.GetPlayerCharacter` 0)))
  (`/Game/blueprint/ui/item/Inventory.AddToInventory` (`/Game/blueprint/character/BP_FirstPersonCharacter.invenwidget` _asbp_first_person_character) (`self.Iteminfo`))
  (`self.K2_DestroyActor`))

(event `UseItem`
  (`KismetSystemLibrary.PrintString` "UseItem1"))

(event `self.ReceiveTick`
  (params (DeltaSeconds :type "Float (single-precision)"))
  (`SceneComponent.K2_AddLocalRotation` (`self.DefaultSceneRoot`) (`KismetMathLibrary.MakeRotator` 0.0 0.0 (+ DeltaSeconds 1.0)) false false))

(fn `UserConstructionScript`
  (`parent.UserConstructionScript`))